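; GA_FireBolt is the Fire Bolt gameplay ability, which casts a projectile toward the target data under the mouse.
; It stores the hit location, draws a debug sphere there, and tells the avatar to update its facing toward it.
; It plays the cast montage, waits for the montage's gameplay event to spawn the projectile, then ends after a short delay.
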(event `self.K2_ActivateAbility`
  (bind (_asynctaskproxy _datahandle) (`TargetDataUnderMouse.CreateTargetDataUnderMouse`)
    (:`ValidData`
      (bind (_bblockinghit _binitialoverlap _time _distance _location) (`GameplayStatics.BreakHitResult` (`AbilitySystemBlueprintLibrary.GetHitResultFromTargetData` _datahandle)))
      (set `self.TargetLocation` _location)
      (`KismetSystemLibrary.DrawDebugSphere` _location 10.0 12 (struct :`R` 1.0 :`G` 0.558934 :`A` 1.0) 1.0 1.0)
      (message `CombatInterface.UpdateFacingTarget` (`self.GetAvatarActorFromActorInfo`) (`self.TargetLocation`))
      (`AbilityTask_PlayMontageAndWait.CreatePlayMontageAndWaitProxy` "None" "/Game/Assets/Characters/Aura/Animations/Abilities/AM_Cast_FireBolt.AM_Cast_FireBolt"
        (:`then`
          (`AbilityTask_WaitGameplayEvent.WaitGameplayEvent` (struct :`TagName` "Event.Montage.FireBolt") null
            (:`EventReceived`
              (`self.SpawnProjectile` (`self.TargetLocation`))
              (`KismetSystemLibrary.Delay` 0.5)
              (`self.K2_EndAbility`))))))))